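; GA_AOETest is a test gameplay ability for a delayed area-of-effect attack centered on the Hawnmun character.
; On activation it caches the mesh's Root socket location and spawns a Niagara effect there, then waits three seconds.
; It then spawns a scaled explosion at the cached spot, damages live players within a fixed radius except ignored actors, and ends the ability.
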(event Ability|EventActivateAbility
  (bind _output_get (Variables|Default|SetCachedPlayerLocation (Transformation|GetSocketLocation (Variables|/Script/Engine.Character|GetMesh (Class|HawnmunGameplayAbility|GetHawnmunCharacterfromActorInfo)) "Root")))
  (Niagara|SpawnSystematLocation "/Game/Assets/KTP_Effect/Particles/Bottom/Bottom06-05.Bottom06-05" _output_get)
  (Utilities|FlowControl|Delay 3.0)
  (Niagara|SpawnSystematLocation "/Game/Assets/KTP_Effect/Particles/Fly/Expolison_08_09.Expolison_08_09" (Variables|Default|GetCachedPlayerLocation) "90.000000,0.000000,0.000000" "2.000000,2.000000,2.000000")
  (bind _outoverlappingactors (Class|HawnmunFunctionLibrary|GetLivePlayersWithinRadius (Class|HawnmunGameplayAbility|GetHawnmunCharacterfromActorInfo) (Variables|Default|GetActors%20to%20Ignore) 5e+02 (Variables|Default|GetCachedPlayerLocation)))
  (for _array_element _outoverlappingactors
    (Class|HawnmunGameplayAbility|CauseDamage _array_element))
  (Ability|EndAbility))
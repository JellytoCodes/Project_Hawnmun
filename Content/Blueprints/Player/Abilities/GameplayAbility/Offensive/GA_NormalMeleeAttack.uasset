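; Gameplay ability for the player's normal melee attack, cycling through a three-montage combo.
; Each activation scales damage from a cached base by combo step and passes damage effect params to the character.
; If an attribute check passes, it commits, plays the montage and advances the step, blocking stamina regen and input via loose tags.
; Montage end clears the tags, ends the ability and starts a short combo-reset timer, cancelled by reactivation.
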(event Custom|ResetCombo
  (Variables|Default|SetLoopMontage 0))

(event Ability|EventActivateAbility
  (bind _returnvalue (Class|HawnmunGameplayAbility|GetHawnmunCharacterfromActorInfo))
  (bind _returnvalue_2 (Class|HawnmunGameplayAbility|GetHawnmunCharacterfromActorInfo))
  (Utilities|Time|ClearandInvalidateTimerbyHandle (Variables|Default|GetComboResetTimer))
  (CallFunction|CalcComboDamage)
  (Variables|/Script/ProjectH.HawnmunCharacterBase|SetCombatDamageEffectParams (Class|HawnmunGameplayAbility|GetHawnmunCharacterfromActorInfo) (Class|HawnmunGameplayAbility|MakeDamageEffectParamsfromClassDefaults 0))
  (if (> (.ReturnValue (Ability|Attribute|GetFloatAttributefromAbilitySystemComponent (Class|HawnmunGameplayAbility|GetHawnmunAbilitySystemComponentfromActorInfo) "(AttributeName=\"Stamina\",Attribute=/Script/ProjectH.HawnmunAttributeSet:Stamina,AttributeOwner=\"/Script/CoreUObject.Class'/Script/ProjectH.HawnmunAttributeSet'\")")) 1.0)
    (Ability|CommitAbility)
    (Ability|GameplayEffect|AddLooseGameplayTags _returnvalue_2 (Variables|Default|GetStaminaRegenBlockedTag))
    (Ability|GameplayEffect|AddLooseGameplayTags _returnvalue_2 (Variables|Default|GetInputLocked))
    (|PlayMontageandWaitProxy "None" (Utilities|Array|Get(acopy) (Variables|Default|GetMontage%20to%20Play) (Variables|Default|GetLoopMontage)) 1.0 "None" true 1.0 0.0 false
      (:then
        (bind _result (Math|Integer|IncrementInt (Variables|Default|GetLoopMontage))
          (:%20%20
            (if (>= _result 3)
              (Variables|Default|SetLoopMontage 0)))))
      (:OnBlendOut
        (Ability|GameplayEffect|RemoveGameplayTags _returnvalue (Variables|Default|GetStaminaRegenBlockedTag) :!label _label)
        (Ability|GameplayEffect|RemoveGameplayTags _returnvalue (Variables|Default|GetInputLocked))
        (Ability|EndAbility)
        (bind _returnvalue_3 (Utilities|Time|SetTimerbyEvent (delegate Custom|ResetCombo) 0.4))
        (Variables|Default|SetComboResetTimer _returnvalue_3))
      (:OnInterrupted
        (goto _label))
      (:OnCancelled
        (goto _label)))
    (else
      (Ability|EndAbility))))

(fn CalcComboDamage
  (bind _loopmontage (Variables|Default|GetLoopMontage))
  (if (> (Variables|Default|GetBaseDamage) 0.0)
    (if (== _loopmontage 0)
      (Variables|Default|SetDamage (Variables|Default|GetBaseDamage))
      (elif (== _loopmontage 1)
        (Variables|Default|SetDamage (* (Variables|Default|GetBaseDamage) 1.2))
        (elif (== _loopmontage 2)
          (Variables|Default|SetDamage (* (Variables|Default|GetBaseDamage) 1.5)))))
    (else
      (Variables|Default|SetBaseDamage (Variables|Default|GetDamage)))))
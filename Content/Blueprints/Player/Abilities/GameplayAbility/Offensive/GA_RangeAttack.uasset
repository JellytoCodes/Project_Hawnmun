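; Gameplay ability for the player's ranged attack, firing a projectile that costs equipped ammo.
; On activation it sets the character's combat damage params, then waits for input press to commit, lock input and play the attack montage.
; The montage's Fire event spends ammo and, if successful, spawns a projectile from MuzzleSocket along actor forward.
; Montage completion or blend-out ends the ability, whose end event removes the input lock.
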(event Ability|EventActivateAbility
  (bind _returnvalue (Ability|GetAvatarActorfromActorInfo))
  (bind _ashawnmun_player_state (Utilities|Casting|CastToHawnmunPlayerState (Game|GetPlayerState 0)))
  (Variables|/Script/ProjectH.HawnmunCharacterBase|SetCombatDamageEffectParams (Class|HawnmunGameplayAbility|GetHawnmunCharacterfromActorInfo) (Class|HawnmunGameplayAbility|MakeDamageEffectParamsfromClassDefaults 0))
  (Ability|Tasks|WaitInputPress false
    (:OnPress
      (Ability|CommitAbility)
      (Ability|GameplayEffect|AddLooseGameplayTags (Class|HawnmunGameplayAbility|GetHawnmunCharacterfromActorInfo) (Variables|Default|GetInputLocked))
      (|PlayMontageandWaitProxy "None" "/Game/Blueprints/Player/AnimMontage/AM_RangeAttack.AM_RangeAttack" 1.0 "None" true 1.0 0.0 false
        (:then
          (Ability|Tasks|WaitGameplayEvent "(TagName=\"Event.Player.Montage.Fire\")" 0
            (:EventReceived
              (bind _returnvalue_2 (Class|HawnmunPlayerState|UseEquippedAmmo _ashawnmun_player_state))
              (if _returnvalue_2
                (bind _returnvalue_3 (Class|CombatInterface|GetProjectileSpawnSocketLocation(Message) _returnvalue "MuzzleSocket"))
                (Class|HawnmunProjectileAbility|SpawnProjectile (+ _returnvalue_3 (* (Transformation|GetActorForwardVector _returnvalue) 1e+03)) "MuzzleSocket" false 0.0)))))
        (:OnCompleted
          (Ability|EndAbility :!label _label))
        (:OnBlendOut
          (goto _label))))))

(event Ability|EventOnEndAbility
  (params (bWasCancelled :type Boolean))
  (Ability|GameplayEffect|RemoveLooseGameplayTags (Class|HawnmunGameplayAbility|GetHawnmunCharacterfromActorInfo) (Variables|Default|GetInputLocked)))
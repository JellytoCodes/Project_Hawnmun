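; GA_Roll is the player's roll gameplay ability, playing a directional roll montage.
; After a brief delay, it ends unless an ability-system attribute exceeds a threshold; otherwise it commits and computes roll direction and distance.
; RollSection selects the forward, backward, left or right montage.
; Loose tags block stamina regen and lock input until the montage blends out, is interrupted or is cancelled, which ends the ability.
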(event Ability|EventActivateAbility
  (bind _returnvalue (Class|HawnmunGameplayAbility|GetHawnmunCharacterfromActorInfo))
  (bind _returnvalue_2 (Class|HawnmunGameplayAbility|GetHawnmunCharacterfromActorInfo))
  (Utilities|FlowControl|Delay 0.05)
  (if (> (.ReturnValue (Ability|Attribute|GetFloatAttributefromAbilitySystemComponent (Class|HawnmunGameplayAbility|GetHawnmunAbilitySystemComponentfromActorInfo) "(AttributeName=\"Stamina\",Attribute=/Script/ProjectH.HawnmunAttributeSet:Stamina,AttributeOwner=\"/Script/CoreUObject.Class'/Script/ProjectH.HawnmunAttributeSet'\")")) 1.0)
    (Ability|CommitAbility)
    (Class|GameplayAbilityRolling|ComputeRollDirectionandDistance)
    (Ability|GameplayEffect|AddLooseGameplayTags _returnvalue_2 (Variables|Default|GetStaminaRegenBlockedTag))
    (Ability|GameplayEffect|AddLooseGameplayTags _returnvalue_2 (Variables|Default|GetInputLockedTag))
    (|PlayMontageandWaitProxy "None" (Utilities|Select :Index (Variables|Default|GetRollSection) :Forward "/Game/Blueprints/Player/AnimMontage/AM_Roll_Forward.AM_Roll_Forward" :Backward "/Game/Blueprints/Player/AnimMontage/AM_Roll_Backword.AM_Roll_Backword" :Left "/Game/Blueprints/Player/AnimMontage/AM_Roll_Left.AM_Roll_Left" :Right "/Game/Blueprints/Player/AnimMontage/AM_Roll_Right.AM_Roll_Right" :End 0) 1.0 "None" true 1.0 0.0 false
      (:OnBlendOut
        _)
      (:OnInterrupted
        _)
      (:OnCancelled
        _))
    (Ability|GameplayEffect|RemoveGameplayTags _returnvalue (Variables|Default|GetStaminaRegenBlockedTag))
    (Ability|GameplayEffect|RemoveGameplayTags _returnvalue (Variables|Default|GetInputLockedTag))
    (Ability|EndAbility)
    (else
      (Ability|EndAbility))))

(event Ability|EventOnEndAbility
  (params (bWasCancelled :type Boolean)))
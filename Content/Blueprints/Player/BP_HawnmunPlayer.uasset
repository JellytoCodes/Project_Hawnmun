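; Hawnmun player character Blueprint that handles the sprint effect and the death-to-mission-fail sequence.
; BeginPlay spawns an inactive anime running Niagara effect, which Tick toggles from the sprinting state and moves to the actor's transform.
; DieEvent disables the input mapping, plays the death montage, pauses animation on completion or blend-out, fades toward black, then shows the cursor and mission-fail widget.
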(event EventDieEvent
  ;[1 0 0] Die Event
  (Class|PlayerInterface|DisableMappingContext)
  (Animation|Montage|PlayMontage (Variables|Character|GetMesh) "/Game/Blueprints/Player/AnimMontage/AM_Death.AM_Death"
    (:OnCompleted
      _)
    (:OnBlendOut
      _))
  (Variables|/Script/Engine.SkeletalMeshComponent|SetbPauseAnims (Variables|Character|GetMesh) true)
  (CameraFades|StartCameraFade (Game|GetPlayerCameraManager 0) 0.0 0.7 1.0 "(R=0.000000,G=0.000000,B=0.000000,A=1.000000)" false true)
  (Utilities|FlowControl|Delay 1.0)
  (bind _ashawnmun_player_controller (Utilities|Casting|CastToHawnmunPlayerController (Pawn|GetController)))
  (Variables|/Script/Engine.PlayerController|SetbShowMouseCursor _ashawnmun_player_controller true)
  (Input|SetInputModeGameandUI _ashawnmun_player_controller 0 "DoNotLock" false false)
  (bind _returnvalue (UserInterface|CreateWidget "/Game/Blueprints/HUD/Mission/WBP_MissionFail.WBP_MissionFail_C"))
  (UserInterface|Viewport|AddtoViewport _returnvalue 0))

(event EventTick
  (params (DeltaSeconds :type Float%20%28single-precision%29))
  (bind _sprintingeffect (Variables|Default|GetSprintingEffect))
  (Utilities|FlowControl|Sequence
    (:then_0
      (if (Class|HawnmunPlayer|GetIsSprinting)
        (Components|Activation|SetActive _sprintingeffect true true)
        (Transformation|SetRelativeLocationAndRotation _sprintingeffect (Transformation|GetActorLocation) (Transformation|GetActorRotation) false false)
        (else
          (Components|Activation|SetActive _sprintingeffect false true))))))

(event EventBeginPlay
  (bind _returnvalue (Niagara|SpawnSystematLocation "/Game/Assets/Effects/sA_Megafxpack_6/sA_MixedVfxpack_4/Fx/NS_Anime_Runnin.NS_Anime_Runnin" "0, 0, 0" "0, 0, 0" "5.000000,5.000000,5.000000" false false))
  (Variables|Default|SetSprintingEffect _returnvalue))

(fn ConstructionScript)
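; Phase 2 gameplay ability for the Nine-Tailed enemy that performs a combo of portal bite and portal breath attacks.
; It plays the combo montage and listens in parallel for its bite and breath gameplay events.
; Bite triggers the boss's portal bite pattern at the player's location and breath activates its portal breath, both using class-default damage params.
; Each then waits on a SkillEnd event with nothing attached; only montage completion ends the ability.
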(event Ability|EventActivateAbility
  (bind _returnvalue (Class|HawnmunGameplayAbility|MakeDamageEffectParamsfromClassDefaults 0))
  (bind _ashawnmun_nine_tailed (Utilities|Casting|CastToHawnmunNineTailed (Class|HawnmunGameplayAbility|GetHawnmunEnemyfromActorInfo)))
  (|PlayMontageandWaitProxy "None" "/Game/Blueprints/Enemy/NineTailed/AnimMontage/Phase2/AM_PortalBreathCombo.AM_PortalBreathCombo" 1.0 "None" true 1.0 0.0 false
    (:then
      (Utilities|FlowControl|Sequence
        (:then_0
          (Ability|Tasks|WaitGameplayEvent "(TagName=\"Event.NineTailed.Montage.PortalBite\")" 0
            (:EventReceived
              (Class|HawnmunNineTailed|ActivePortalBitePattern _ashawnmun_nine_tailed (Transformation|GetActorLocation (Game|Player|GetPlayerPawn 0)) _returnvalue 1 0.5))))
        (:then_1
          (Ability|Tasks|WaitGameplayEvent "(TagName=\"Event.NineTailed.Montage.PortalBreath\")" 0
            (:EventReceived
              (Class|HawnmunNineTailed|ActivePortalBreath _ashawnmun_nine_tailed 2 _returnvalue)))))
      (Ability|Tasks|WaitGameplayEvent "(TagName=\"Event.Combat.SkillEnd\")" 0))
    (:OnCompleted
      (Ability|EndAbility))))
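; Gameplay ability for the Nine-Tailed enemy's charm illusion attack.
; Runs a fixed chain of delays that delegates each phase to BP_NineTailed: charm effect, illusion shuffle, effects off during a longer wait, then effects back on.
; It finishes by calling BackCenterLocation with damage effect params built from the ability's class defaults, then clears the charm effect and ends.
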(event Ability|EventActivateAbility
  (bind _asbp_nine_tailed (Utilities|Casting|CastToBP_NineTailed (Class|HawnmunGameplayAbility|GetHawnmunEnemyfromActorInfo)))
  (bind _output_get (Variables|Default|SetOwnerActor _asbp_nine_tailed))
  (Class|HawnmunNineTailed|ActivateCharmIllusionEffect _output_get)
  (Utilities|FlowControl|Delay 5.0)
  (Class|HawnmunNineTailed|ShuffleNineTailedCharmIllusion (Variables|Default|GetOwnerActor))
  (Utilities|FlowControl|Delay 0.5)
  (Class|HawnmunNineTailed|DeactivateCharmIllusionEffect (Variables|Default|GetOwnerActor))
  (Class|HawnmunNineTailed|DeactivateIllusionsEffect (Variables|Default|GetOwnerActor))
  (Utilities|FlowControl|Delay 1e+01)
  (Class|HawnmunNineTailed|ActivateCharmIllusionEffect (Variables|Default|GetOwnerActor))
  (Class|HawnmunNineTailed|ActivateIllusionsEffect (Variables|Default|GetOwnerActor))
  (Utilities|FlowControl|Delay 5.0)
  (Class|HawnmunNineTailed|BackCenterLocation (Variables|Default|GetOwnerActor) (Class|HawnmunGameplayAbility|MakeDamageEffectParamsfromClassDefaults 0))
  (Utilities|FlowControl|Delay 1.0)
  (Class|HawnmunNineTailed|DeactivateCharmIllusionEffect (Variables|Default|GetOwnerActor))
  (Ability|EndAbility))
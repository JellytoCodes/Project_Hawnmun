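; Illusion actor for the Nine-Tailed enemy, handling the visual and audio effects of its charm illusion.
; Activate and deactivate events each run a timeline that drives the dissolve value, with the charm effect active until it finishes.
; Deactivation also starts a show montage alongside the dissolve and re-enables tail and ear effects at the end.
; A damage-effect event spawns a fire Niagara burst and explosion sound at the actor's location.
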(event EventCauseDamageEffect
  (bind _returnvalue (Transformation|GetActorTransform))
  (Niagara|SpawnSystematLocation "/Game/Assets/Effects/FireVFX/Niagaras/Basic/NS_powerup_fire.NS_powerup_fire" (.location _returnvalue) (.rotation _returnvalue) (.scale _returnvalue))
  (Audio|PlaySoundatLocation "/Game/Assets/Sound/NineTailedSound/SFX_Illusion_Explosion.SFX_Illusion_Explosion" (Transformation|GetActorLocation) "0, 0, 0" 1.0 1.0 0.0 0 0 0 0))

(event EventActivateCharmIllusionEffect
  (Components|Activation|SetActive (Variables|Default|GetCharmIllusionEffect) true true)
  (bind _animation (Timeline|ActivateIllusion PlayFromStart)
    (:Update
      (Class|HawnmunNineTailedIllusion|SetCharmIllusionDissolveValue _animation))
    (:Finished
      (Components|Activation|SetActive (Variables|Default|GetCharmIllusionEffect) false false))))

(event EventDeactivateCharmIllusionEffect
  (Components|Activation|SetActive (Variables|Default|GetCharmIllusionEffect) true false)
  (Animation|Montage|PlayMontage (Variables|Character|GetMesh) "/Game/Blueprints/Enemy/NineTailed/AnimMontage/Phase1/AM_NineTailed_CharmIllusion_Show.AM_NineTailed_CharmIllusion_Show"
    (:then
      (bind _animation (Timeline|DeactivateIllusion PlayFromStart)
        (:Update
          (Class|HawnmunNineTailedIllusion|SetCharmIllusionDissolveValue _animation))
        (:Finished
          (Components|Activation|SetActive (Variables|Default|GetCharmIllusionEffect) false false)
          (Class|HawnmunNineTailedIllusion|SetTailEarEffectsActive true))))))

(fn ConstructionScript)
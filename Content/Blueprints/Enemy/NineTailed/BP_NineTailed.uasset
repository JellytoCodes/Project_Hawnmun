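; BP_NineTailed is the Blueprint for the Nine-Tailed enemy, handling its combat facing, charm illusion visuals and death animation.
; Facing updates set a "CombatTarget" motion warping target at the given location.
; Charm illusion activation and deactivation play a particle effect, cast sound and timeline-driven dissolve, with deactivation re-enabling tail and ear effects when finished.
; Death plays a montage and pauses mesh animations on blend out.
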(event EventUpdateFacingTarget
  (params (Target :type Vector%20%28by%20ref%29 :default "0, 0, 0"))
  (Class|MotionWarpingComponent|AddorUpdateWarpTargetfromLocation (Variables|Default|GetMotionWarpingComponent) "CombatTarget" Target))

(event EventActivateCharmIllusionEffect
  (Components|Activation|SetActive (Variables|Default|GetCharmIllusionEffect) true true)
  (Audio|PlaySoundatLocation "/Game/Assets/Sound/NineTailedSound/SFX_Illusion_Cast.SFX_Illusion_Cast" (Transformation|GetActorLocation) "0, 0, 0" 1.0 1.0 0.0 0 0 0 0)
  (bind _animation (Timeline|ActivateIllusion PlayFromStart)
    (:Update
      (Class|HawnmunNineTailed|SetCharmIllusionDissolveValue _animation))
    (:Finished
      (Components|Activation|SetActive (Variables|Default|GetCharmIllusionEffect) false false))))

(event EventDeactivateCharmIllusionEffect
  (Components|Activation|SetActive (Variables|Default|GetCharmIllusionEffect) true true)
  (Audio|PlaySoundatLocation "/Game/Assets/Sound/NineTailedSound/SFX_Illusion_Cast.SFX_Illusion_Cast" (Transformation|GetActorLocation) "0, 0, 0" 1.0 1.0 0.0 0 0 0 0)
  (bind _animation (Timeline|DeactivateIllusion PlayFromStart)
    (:Update
      (Class|HawnmunNineTailed|SetCharmIllusionDissolveValue _animation))
    (:Finished
      (Components|Activation|SetActive (Variables|Default|GetCharmIllusionEffect) false false)
      (Class|HawnmunNineTailed|SetTailEarEffectsActive true))))

(event EventDieEvent
  (Animation|Montage|PlayMontage (Variables|Character|GetMesh) "/Game/Blueprints/Enemy/NineTailed/AnimMontage/AM_Dead.AM_Dead"
    (:OnBlendOut
      (Variables|/Script/Engine.SkeletalMeshComponent|SetbPauseAnims (Variables|Character|GetMesh) true))))

(fn ConstructionScript)
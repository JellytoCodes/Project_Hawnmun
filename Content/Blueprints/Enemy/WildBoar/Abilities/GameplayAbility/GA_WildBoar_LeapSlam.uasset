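; Wild boar enemy gameplay ability that performs a leap slam, damaging live players around the landing.
; On activation it updates the boar's facing target to player 0's location and plays the leap slam montage.
; Montage gameplay events launch the boar upward, drive it hard down, then trigger radial damage centered on the left foot socket.
; The ability ends when the montage completes.
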(event Ability|EventActivateAbility
  (Utilities|FlowControl|Sequence
    (:then_0
      (Ability|Tasks|WaitGameplayEvent "(TagName=\"Event.Montage.TakeOff\")" 0
        (:then
          (Class|CombatInterface|UpdateFacingTarget(Message) (Class|HawnmunGameplayAbility|GetHawnmunEnemyfromActorInfo) (Transformation|GetActorLocation (Game|Player|GetPlayerPawn 0))))))
    (:then_1
      (|PlayMontageandWaitProxy "None" "/Game/Blueprints/Enemy/WildBoar/AnimMontage/AM_LeapSlam.AM_LeapSlam" 1.0 "None" true 1.0 0.0 false
        (:then
          (Utilities|FlowControl|Sequence
            (:then_0
              (Ability|Tasks|WaitGameplayEvent "(TagName=\"Event.Montage.TakeOff\")" 0
                (:EventReceived
                  (Character|LaunchCharacter (Class|HawnmunGameplayAbility|GetHawnmunEnemyfromActorInfo) "0.000000,0.000000,1200.000000" false true))))
            (:then_1
              (Ability|Tasks|WaitGameplayEvent "(TagName=\"Event.Montage.SlamDown\")" 0
                (:EventReceived
                  (Character|LaunchCharacter (Class|HawnmunGameplayAbility|GetHawnmunEnemyfromActorInfo) "0.000000,0.000000,-8000.000000" false true))))
            (:then_2
              (Ability|Tasks|WaitGameplayEvent "(TagName=\"Event.WildBoar.Montage.LeapSlam\")" 0
                (:EventReceived
                  (CallFunction|ApplyDamage))))))
        (:OnCompleted
          (Ability|EndAbility))))))

(fn ApplyDamage
  (Variables|Default|SetRadialDamageOrigin (Transformation|GetSocketLocation (Variables|/Script/Engine.Character|GetMesh (Class|HawnmunGameplayAbility|GetHawnmunEnemyfromActorInfo)) "foot_l"))
  (Variables|/Script/ProjectH.HawnmunCharacterBase|SetCombatDamageEffectParams (Class|HawnmunGameplayAbility|GetHawnmunEnemyfromActorInfo) (Class|HawnmunGameplayAbility|MakeDamageEffectParamsfromClassDefaults 0))
  (bind _outoverlappingactors (Class|HawnmunFunctionLibrary|GetLivePlayersWithinRadius self (Utilities|Array|MakeArray (Class|HawnmunGameplayAbility|GetHawnmunEnemyfromActorInfo)) (Variables|Default|GetRadialDamageOuterRadius) (Variables|Default|GetRadialDamageOrigin)))
  (bind _output_get (Variables|Default|SetOut%20Overlapping%20Actors _outoverlappingactors))
  (for _array_element _output_get
    (Class|HawnmunGameplayAbility|CauseDamage _array_element)))
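; Gameplay ability for the Wild Boar enemy's foot stomp, a repeated area attack that damages nearby players.
; On activation it turns the boar toward the first player once, then replays the stomp montage a random number of times.
; Each montage's gameplay event triggers damage to live players within a radius of the left foot socket, using damage parameters from class defaults.
; The ability ends when the final montage completes.
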(event Custom|ExecuteStomp
  (|PlayMontageandWaitProxy "None" "/Game/Blueprints/Enemy/WildBoar/AnimMontage/AM_FootStomp.AM_FootStomp" 1.0 "None" true 1.0 0.0 false
    (:then
      (Ability|Tasks|WaitGameplayEvent "(TagName=\"Event.WildBoar.Montage.FootStomp\")" 0
        (:EventReceived
          (CallFunction|ApplyDamage))))
    (:OnCompleted
      (if (> (Variables|Default|GetRemainStompCount) 0)
        (Math|Integer|DecrementInt (Variables|Default|GetRemainStompCount)
          (:%20%20
            (CallFunction|ExecuteStomp)))
        (else
          (Ability|EndAbility))))))

(event Ability|EventActivateAbility
  (Variables|Default|SetRemainStompCount (Math|Random|RandomIntegerinRange 2 4))
  (Class|CombatInterface|UpdateFacingTarget(Message) (Class|HawnmunGameplayAbility|GetHawnmunEnemyfromActorInfo) (Transformation|GetActorLocation (Game|Player|GetPlayerPawn 0)))
  (CallFunction|ExecuteStomp))

(fn ApplyDamage
  (Variables|Default|SetRadialDamageOrigin (Transformation|GetSocketLocation (Variables|/Script/Engine.Character|GetMesh (Class|HawnmunGameplayAbility|GetHawnmunEnemyfromActorInfo)) "foot_l"))
  (Variables|/Script/ProjectH.HawnmunCharacterBase|SetCombatDamageEffectParams (Class|HawnmunGameplayAbility|GetHawnmunEnemyfromActorInfo) (Class|HawnmunGameplayAbility|MakeDamageEffectParamsfromClassDefaults 0))
  (bind _outoverlappingactors (Class|HawnmunFunctionLibrary|GetLivePlayersWithinRadius self (Utilities|Array|MakeArray (Class|HawnmunGameplayAbility|GetHawnmunEnemyfromActorInfo)) (Variables|Default|GetRadialDamageOuterRadius) (Variables|Default|GetRadialDamageOrigin)))
  (bind _output_get (Variables|Default|SetOut%20Overlapping%20Actors _outoverlappingactors))
  (for _array_element _output_get
    (Class|HawnmunGameplayAbility|CauseDamage _array_element)))
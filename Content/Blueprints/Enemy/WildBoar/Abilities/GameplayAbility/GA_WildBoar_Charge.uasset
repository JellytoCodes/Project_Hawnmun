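; Gameplay ability for the Wild Boar enemy's charge attack against the player, played as start, charge and end montages.
; After the wind-up blends out, it re-faces the player and applies a constant root motion force along that direction while the charge montage plays.
; When the force finishes, the end montage plays, and its gameplay event triggers radial damage to live players around the hand_l socket.
; The ability ends when that montage completes.
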(event Ability|EventActivateAbility
  (bind _returnvalue (Game|Player|GetPlayerPawn 0))
  (bind _returnvalue_2 (Transformation|GetActorLocation _returnvalue))
  (Class|CombatInterface|UpdateFacingTarget(Message) (Class|HawnmunGameplayAbility|GetHawnmunEnemyfromActorInfo) (Transformation|GetActorLocation (Game|Player|GetPlayerPawn 0)))
  (|PlayMontageandWaitProxy "None" "/Game/Blueprints/Enemy/WildBoar/AnimMontage/AM_Charge_Start.AM_Charge_Start" 1.0 "None" true 1.0 0.0 false
    (:OnBlendOut
      (Utilities|FlowControl|Sequence
        (:then_0
          (Class|CombatInterface|UpdateFacingTarget(Message) (Class|HawnmunGameplayAbility|GetHawnmunEnemyfromActorInfo) _returnvalue_2)
          (|PlayMontageandWaitProxy "None" "/Game/Blueprints/Enemy/WildBoar/AnimMontage/AM_Charge.AM_Charge" 1.0 "None" true 1.0 0.0 false))
        (:then_1
          (Ability|Tasks|ApplyRootMotionConstantForce "None" (Math|Vector|GetUnitDirection(Vector) (Transformation|GetActorLocation (Ability|GetAvatarActorfromActorInfo)) _returnvalue_2) 1.8e+03 1.2 false 0 "MaintainLastRootMotionVelocity" "0, 0, 0" 0.0 true
            (:OnFinish
              (|PlayMontageandWaitProxy "None" "/Game/Blueprints/Enemy/WildBoar/AnimMontage/AM_Charge_End.AM_Charge_End" 1.0 "None" true 1.0 0.0 false
                (:then
                  (Ability|Tasks|WaitGameplayEvent "(TagName=\"Event.WildBoar.Montage.Charge\")" 0
                    (:EventReceived
                      (CallFunction|ApplyDamage))))
                (:OnCompleted
                  (Ability|EndAbility))))))))))

(fn ApplyDamage
  (Variables|Default|SetRadialDamageOrigin (Transformation|GetSocketLocation (Variables|/Script/Engine.Character|GetMesh (Class|HawnmunGameplayAbility|GetHawnmunEnemyfromActorInfo)) "hand_l"))
  (Variables|/Script/ProjectH.HawnmunCharacterBase|SetCombatDamageEffectParams (Class|HawnmunGameplayAbility|GetHawnmunEnemyfromActorInfo) (Class|HawnmunGameplayAbility|MakeDamageEffectParamsfromClassDefaults 0))
  (bind _outoverlappingactors (Class|HawnmunFunctionLibrary|GetLivePlayersWithinRadius self (Utilities|Array|MakeArray (Class|HawnmunGameplayAbility|GetHawnmunEnemyfromActorInfo)) (Variables|Default|GetRadialDamageOuterRadius) (Variables|Default|GetRadialDamageOrigin)))
  (bind _output_get (Variables|Default|SetOut%20Overlapping%20Actors _outoverlappingactors))
  (for _array_element _output_get
    (Class|HawnmunGameplayAbility|CauseDamage _array_element)))
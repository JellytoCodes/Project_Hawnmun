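; Wild Boar enemy gameplay ability for a double slam attack that deals radial damage.
; On activation it turns the boar toward player 0's location and plays the slam montage, ending when the montage completes.
; A montage gameplay event triggers damage to live players within the outer radius of the left-hand socket, using effect params from class defaults.
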(event Ability|EventActivateAbility
  (Class|CombatInterface|UpdateFacingTarget(Message) (Class|HawnmunGameplayAbility|GetHawnmunEnemyfromActorInfo) (Transformation|GetActorLocation (Game|Player|GetPlayerPawn 0)))
  (|PlayMontageandWaitProxy "None" "/Game/Blueprints/Enemy/WildBoar/AnimMontage/AM_DoubleSlam.AM_DoubleSlam" 1.0 "None" true 1.0 0.0 false
    (:then
      (Ability|Tasks|WaitGameplayEvent "(TagName=\"Event.WildBoar.Montage.DoubleSlam\")" 0
        (:EventReceived
          (CallFunction|ApplyDamage))))
    (:OnCompleted
      (Ability|EndAbility))))

(fn ApplyDamage
  (Variables|Default|SetRadialDamageOrigin (Transformation|GetSocketLocation (Variables|/Script/Engine.Character|GetMesh (Class|HawnmunGameplayAbility|GetHawnmunEnemyfromActorInfo)) "hand_l"))
  (Variables|/Script/ProjectH.HawnmunCharacterBase|SetCombatDamageEffectParams (Class|HawnmunGameplayAbility|GetHawnmunEnemyfromActorInfo) (Class|HawnmunGameplayAbility|MakeDamageEffectParamsfromClassDefaults 0))
  (bind _outoverlappingactors (Class|HawnmunFunctionLibrary|GetLivePlayersWithinRadius self (Utilities|Array|MakeArray (Class|HawnmunGameplayAbility|GetHawnmunEnemyfromActorInfo)) (Variables|Default|GetRadialDamageOuterRadius) (Variables|Default|GetRadialDamageOrigin)))
  (bind _output_get (Variables|Default|SetOut%20Overlapping%20Actors _outoverlappingactors))
  (for _array_element _output_get
    (Class|HawnmunGameplayAbility|CauseDamage _array_element)))
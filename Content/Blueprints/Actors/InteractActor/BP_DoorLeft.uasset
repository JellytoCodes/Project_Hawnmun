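; BP_DoorLeft is an interactable left door actor whose barrier breaks open with a cinematic.
; OpenDoorEvent shows the cinematic widget on the HawnmunHUD and requests the Cinematic.BreakBarrier cinematic through its slot widget controller.
; It then deactivates the Niagara effect and instantly rotates DoorMesh 80 degrees in yaw, without a timeline or interpolation.
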(event EventOpenDoorEvent
  (bind _ashawnmun_hud (Utilities|Casting|CastToHawnmunHUD (HUD|GetHUD (Game|GetPlayerController 0))))
  (Class|HawnmunHUD|ShowCinematicWidget _ashawnmun_hud)
  (Class|CinematicWidgetController|RequestPlayCinematic (Class|HawnmunHUD|GetCinematicSlotWidgetController _ashawnmun_hud (Utilities|Struct|MakeWidgetControllerParams)) "(TagName=\"Cinematic.BreakBarrier\")" 0)
  (Components|Activation|Deactivate (Variables|Default|GetNiagara))
  (Transformation|SetWorldRotation (Variables|Default|GetDoorMesh) (Math|Rotator|CombineRotators (Transformation|GetWorldRotation (Variables|Default|GetDoorMesh)) "0.000000,80.000000,0.000000") false false))

(fn ConstructionScript)
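; Portal breath attack actor among the Nine-Tailed actors, which telegraphs and then fires a beam.
; StartChargeAnimation plays a start sound and runs two timelines, one fading in the fox-head Niagara effect and one driving warning decal progress.
; When the decal timeline finishes, it fires the beam with a breathing sound, fades the head out and cancels the breath after a short delay.
; Beam, decal and cancel logic are defined outside this graph.
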(event EventStartChargeAnimation
  (Audio|PlaySoundatLocation "/Game/Assets/Sound/NineTailedSound/SFX_PortalBreath_Start.SFX_PortalBreath_Start" (Transformation|GetActorLocation) "0, 0, 0" 1.0 1.0 0.0 0 0 0 0)
  (Utilities|FlowControl|Sequence
    (:then_0
      (bind _progress (Timeline|Timeline_0 PlayFromStart)
        (:Update
          (Niagara|SetNiagaraVariable(Float) (Variables|Default|GetFoxHeadEffect) "User.Opacity" _progress))))
    (:then_1
      (bind _progress_2 (Timeline|Timeline PlayFromStart)
        (:Update
          (Class|PortalBreathActor|UpdateWarningDecalProgress _progress_2))
        (:Finished
          (Class|PortalBreathActor|FireBeam)
          (Audio|PlaySoundatLocation "/Game/Assets/Sound/NineTailedSound/SFX_PortalBreath_Breathing.SFX_PortalBreath_Breathing" (Transformation|GetActorLocation) "0, 0, 0" 1.0 1.0 0.0 0 0 0 0)
          (Utilities|FlowControl|Sequence
            (:then_0
              (Timeline|Timeline_0 ReverseFromEnd))
            (:then_1
              (Utilities|FlowControl|Delay 2.0)
              (Class|PortalBreathActor|CancelPortalBreath))))))))

(fn ConstructionScript)
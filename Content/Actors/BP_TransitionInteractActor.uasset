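; BP_TransitionInteractActor is a trigger that moves the player to a destination point behind a black screen fade.
; When an actor implementing PlayerInterface overlaps PlatformCollision, Enable turns off its input mapping context through an interface message and fades the camera out.
; Disable then teleports the actor to DestinationPoint with zero rotation, fades back in after a short delay and restores the mapping context.
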(event OnComponentBeginOverlap(PlatformCollision)
  (params (OverlappedComponent :type Primitive%20Component%20Object%20Reference) (OtherActor :type Actor%20Object%20Reference) (OtherComp :type Primitive%20Component%20Object%20Reference) (OtherBodyIndex :type Integer) (bFromSweep :type Boolean) (SweepResult :type Hit%20Result%20Structure%20%28by%20ref%29))
  (Variables|Default|SetOther%20Actor OtherActor)
  (if (Utilities|DoesObjectImplementInterface OtherActor "/Script/ProjectH.PlayerInterface")
    (CallFunction|Enable)))

(event Custom|Disable
  (bind _returnvalue (Game|GetPlayerCameraManager 0))
  (bind _duration (Variables|Default|GetDuration))
  (Transformation|Teleport (Variables|Default|GetOther%20Actor) (Transformation|GetWorldLocation (Variables|Default|GetDestinationPoint)) "0, 0, 0")
  (Utilities|FlowControl|Delay 0.5)
  (CameraFades|StartCameraFade :self _returnvalue :FromAlpha 1.0 :Duration _duration)
  (Utilities|FlowControl|Delay _duration)
  (Class|PlayerCameraManager|SetManualCameraFade :self _returnvalue)
  (Class|PlayerInterface|EnableMappingContext(Message) (Variables|Default|GetOther%20Actor)))

(event Custom|Enable
  (bind _returnvalue (Game|GetPlayerCameraManager 0))
  (bind _duration (Variables|Default|GetDuration))
  (Class|PlayerInterface|DisableMappingContext(Message) (Variables|Default|GetOther%20Actor))
  (CameraFades|StartCameraFade :self _returnvalue :ToAlpha 2.0 :Duration _duration)
  (Utilities|FlowControl|Delay _duration)
  (Class|PlayerCameraManager|SetManualCameraFade :self _returnvalue :InFadeAmount 1.0)
  (CallFunction|Disable))

(fn ConstructionScript)
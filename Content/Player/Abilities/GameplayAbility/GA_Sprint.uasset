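; Gameplay ability for hold-to-sprint on the Hawnmun character, gated by an attribute threshold, likely stamina.
; On activation it commits, raises walk speed, sets the sprinting flag and adds a loose tag blocking stamina regen.
; It ends on input release or when the watched attribute nears zero.
; Ending restores speed, clears the flag and tag, and removes active effects granting Cost.Sprint.
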(event Ability|EventActivateAbility
  (bind _returnvalue (Class|HawnmunGameplayAbility|GetHawnmunCharacterfromActorInfo))
  (Ability|CommitAbility)
  (if (> (.ReturnValue (Ability|Attribute|GetFloatAttributefromAbilitySystemComponent (Class|HawnmunGameplayAbility|GetHawnmunAbilitySystemComponentfromActorInfo) "(AttributeName=\"Stamina\",Attribute=/Script/ProjectH.HawnmunAttributeSet:Stamina,AttributeOwner=\"/Script/CoreUObject.Class'/Script/ProjectH.HawnmunAttributeSet'\")")) 1.0)
    (Ability|Tasks|WaitInputRelease false
      (:then
        (Utilities|FlowControl|Sequence
          (:then_0
            (Ability|GameplayEffect|AddLooseGameplayTags _returnvalue (Variables|Default|GetStaminaRegenBlockedTag))
            (Class|HawnmunPlayer|SetIsSprinting _returnvalue true)
            (Variables|/Script/Engine.CharacterMovementComponent|SetMaxWalkSpeed (Variables|/Script/Engine.Character|GetCharacterMovement _returnvalue) 8e+02))
          (:then_1
            (bind _bmatchescomparison (Ability|Tasks|WaitForAttributeChangeThreshold "(AttributeName=\"Stamina\",Attribute=/Script/ProjectH.HawnmunAttributeSet:Stamina,AttributeOwner=\"/Script/CoreUObject.Class'/Script/ProjectH.HawnmunAttributeSet'\")" "LessThanOrEqualTo" 0.1 false 0)
              (:OnChange
                (if _bmatchescomparison
                  (Ability|EndAbility)))))))
      (:OnRelease
        (Ability|EndAbility :!label _label)))
    (else
      (goto _label))))

(event Ability|EventOnEndAbility
  (params (bWasCancelled :type Boolean))
  (bind _returnvalue (Class|HawnmunGameplayAbility|GetHawnmunCharacterfromActorInfo))
  (Class|HawnmunPlayer|SetIsSprinting _returnvalue false)
  (Variables|/Script/Engine.CharacterMovementComponent|SetMaxWalkSpeed (Variables|/Script/Engine.Character|GetCharacterMovement _returnvalue) 4e+02)
  (GameplayEffects|RemoveActiveEffectswithGrantedTags (Class|HawnmunGameplayAbility|GetHawnmunAbilitySystemComponentfromActorInfo) "(GameplayTags=((TagName=\"Cost.Sprint\")))")
  (Ability|GameplayEffect|RemoveLooseGameplayTags (Class|HawnmunGameplayAbility|GetHawnmunCharacterfromActorInfo) (Variables|Default|GetStaminaRegenBlockedTag)))
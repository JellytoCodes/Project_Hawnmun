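; Gameplay ability for the player's normal melee attack, cycling through a three-montage combo.
; On activation it clears the combo reset timer, checks an attribute minimum, then waits for an input press to commit and play the current montage.
; A loose tag blocks stamina regeneration until the ability ends.
; The combo index advances as each montage starts, and a short timer after it finishes or is interrupted resets the chain.
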(event Custom|CustomEvent
  (Variables|Default|SetLoopMontage 0))

(event Ability|EventActivateAbility
  (Utilities|Time|ClearandInvalidateTimerbyHandle (Variables|Default|GetComboResetTimer))
  (if (> (.ReturnValue (Ability|Attribute|GetFloatAttributefromAbilitySystemComponent (Class|HawnmunGameplayAbility|GetHawnmunAbilitySystemComponentfromActorInfo) "(AttributeName=\"Stamina\",Attribute=/Script/ProjectH.HawnmunAttributeSet:Stamina,AttributeOwner=\"/Script/CoreUObject.Class'/Script/ProjectH.HawnmunAttributeSet'\")")) 1.0)
    (Ability|Tasks|WaitInputPress false
      (:OnPress
        (Ability|CommitAbility)
        (Ability|GameplayEffect|AddLooseGameplayTags (Class|HawnmunGameplayAbility|GetHawnmunCharacterfromActorInfo) (Variables|Default|GetStaminaRegenBlockedTag))
        (|PlayMontageandWaitProxy "None" (Utilities|Array|Get(acopy) (Variables|Default|GetMontage%20to%20Play) (Variables|Default|GetLoopMontage)) 1.0 "None" true 1.0 0.0 false
          (:then
            (Utilities|FlowControl|Sequence
              (:then_0
                (bind _result (Math|Integer|IncrementInt (Variables|Default|GetLoopMontage))
                  (:%20%20
                    (if (>= _result 3)
                      (Variables|Default|SetLoopMontage 0)))))))
          (:OnCompleted
            (Ability|EndAbility :!label _label)
            (bind _returnvalue (Utilities|Time|SetTimerbyEvent (delegate Custom|CustomEvent) 0.4))
            (Variables|Default|SetComboResetTimer _returnvalue))
          (:OnBlendOut
            (goto _label))
          (:OnInterrupted
            (goto _label))
          (:OnCancelled
            (goto _label)))))
    (else
      (Ability|EndAbility))))

(event Ability|EventOnEndAbility
  (params (bWasCancelled :type Boolean))
  (Ability|GameplayEffect|RemoveGameplayTags (Class|HawnmunGameplayAbility|GetHawnmunCharacterfromActorInfo) (Variables|Default|GetStaminaRegenBlockedTag)))